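; BP_GravitronUlt is an ultimate projectile that becomes a temporary gravity well for physics objects.
; After a delay it stops moving, triples its scale, reveals its sphere and starts pulling, then destroys itself when its lifetime ends.
; Overlap events on PhysicsObjectDetection track simulating components in an array.
; While active, Tick applies a negative radial impulse as a velocity change to those components, drawing them toward the actor.
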(event `self.ReceiveBeginPlay`
  (bind _projectilemovement (`self.ProjectileMovement`))
  ;[1 1 1] StopMoving and Allow canCheck
  (`KismetSystemLibrary.Delay` (`self.TimeBeforeGravityPull`))
  (`SceneComponent.SetVisibility` (`self.Sphere`) true false)
  (set `self.CanCheck` true)
  (`MovementComponent.StopMovementImmediately` _projectilemovement)
  (`self.SetActorScale3D` (* (`self.GetActorScale3D`) 3))
  (set `ProjectileMovementComponent.ProjectileGravityScale` 0.0 _projectilemovement)
  (`KismetSystemLibrary.Delay` (`self.Ult Lifetime`))
  (`self.K2_DestroyActor`))

(event `self.PhysicsObjectDetection.OnComponentBeginOverlap`
  (params (OverlappedComponent :type "PrimitiveComponent Object Reference") (OtherActor :type "Actor Object Reference") (OtherComp :type "PrimitiveComponent Object Reference") (OtherBodyIndex :type Integer) (bFromSweep :type Boolean) (SweepResult :type "HitResult Structure (by ref)"))
  ;[1 1 1] Detect Objects and Add or Remove from Array
  (if (`SceneComponent.IsSimulatingPhysics` OtherComp "None")
    (`KismetArrayLibrary.Array_Add` (`self.ObjectsInUltimate`) OtherComp)))

(event `self.PhysicsObjectDetection.OnComponentEndOverlap`
  (params (OverlappedComponent :type "PrimitiveComponent Object Reference") (OtherActor :type "Actor Object Reference") (OtherComp :type "PrimitiveComponent Object Reference") (OtherBodyIndex :type Integer))
  ;[1 1 1] Detect Objects and Add or Remove from Array
  (if (`SceneComponent.IsSimulatingPhysics` OtherComp "None")
    (`KismetArrayLibrary.Array_RemoveItem` (`self.ObjectsInUltimate`) OtherComp)))

(event `self.ReceiveTick`
  (params (DeltaSeconds :type "Float (single-precision)"))
  (bind _objectsinultimate (`self.ObjectsInUltimate`))
  ;[1 1 1] Pull and Move Objects
  (if (`self.CanCheck`)
    (if (>= (`KismetArrayLibrary.Array_LastIndex` _objectsinultimate) 0)
      (`PrimitiveComponent.AddRadialImpulse` _objectsinultimate (`self.K2_GetActorLocation`) 2000.0 -75.0 "RIF_Linear" true))))

(fn `UserConstructionScript`)