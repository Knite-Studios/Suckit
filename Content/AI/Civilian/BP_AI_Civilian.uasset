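; Civilian AI character that fights with punches, takes damage and can be killed by a stealth neck-break takedown.
; Behavior-tree attack calls drive a three-hit montage combo, with timer-looped sphere traces on sockets of the overlapping player's mesh (AIBP) applying damage.
; Hits interrupt combos and launch the character; death ragdolls it.
; Camera-facing widgets show health, takedown prompt and investigate icon, and the takedown returns the assassin's reference transform.
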(event `self.ReceiveBeginPlay`
  (bind _aswb_dummy_health_bar (cast `/Game/ThirdPerson/UI/WB_DummyHealthBar` (`WidgetComponent.GetWidget` (`self.Health Bar Widget`))))
  (set `self.HealthBarUI` _aswb_dummy_health_bar))

(event `self.ReceiveTick`
  (params (DeltaSeconds :type "Float (single-precision)"))
  ;[0.05127 0.05127 0.05127] Widget Rotation
  (`SceneComponent.K2_SetWorldRotation` (`self.Takedown Widget`) (`KismetMathLibrary.FindLookAtRotation` (`SceneComponent.K2_GetComponentLocation` (`self.Takedown Widget`)) (`SceneComponent.K2_GetComponentLocation` (`PlayerCameraManager.TransformComponent` (`GameplayStatics.GetPlayerCameraManager` 0)))) false false)
  (`SceneComponent.K2_SetWorldRotation` (`self.Health Bar Widget`) (`KismetMathLibrary.FindLookAtRotation` (`SceneComponent.K2_GetComponentLocation` (`self.Takedown Widget`)) (`SceneComponent.K2_GetComponentLocation` (`PlayerCameraManager.TransformComponent` (`GameplayStatics.GetPlayerCameraManager` 0)))) false false)
  (`SceneComponent.K2_SetWorldRotation` (`self.Investigate Widget`) (`KismetMathLibrary.FindLookAtRotation` (`SceneComponent.K2_GetComponentLocation` (`self.Takedown Widget`)) (`SceneComponent.K2_GetComponentLocation` (`PlayerCameraManager.TransformComponent` (`GameplayStatics.GetPlayerCameraManager` 0)))) false false))

(event `Ragdoll`
  (bind _bpc_playerstats (`self.BPC_PlayerStats`))
  ;[0.05127 0.05127 0.05127] Ragdoll
  (`/Game/ThirdPerson/Blueprints/BPC_PlayerStats.Decrease Health` _bpc_playerstats (`/Game/ThirdPerson/Blueprints/BPC_PlayerStats.Max Health` _bpc_playerstats))
  (`PrimitiveComponent.SetCollisionObjectType` (`self.Mesh`) "ECC_PhysicsBody")
  (`|ExecutionSequence`
    (:`then_0`
      (`KismetSystemLibrary.Delay` 2.5)
      (`PrimitiveComponent.SetSimulatePhysics` (`self.Mesh`) true)
      (`SceneComponent.SetVisibility` (`self.Health Bar Widget`) false false)
      (`ActorComponent.K2_DestroyComponent` (`self.CapsuleComponent`))
      (`ActorComponent.K2_DestroyComponent` (`self.Assassination Radius`))
      (`CharacterMovementComponent.DisableMovement` (`self.CharacterMovement`)))
    (:`then_1`
      (`KismetSystemLibrary.Delay` 1.4)
      (`GameplayStatics.PlaySoundAtLocation` "/Game/Audio/Grunts-Hits/MS_Death.MS_Death" (`self.K2_GetActorLocation`) (struct) 1.0 1.0 0.0 null null null null))))

(event `self.Assassination Radius.OnComponentBeginOverlap`
  (params (OverlappedComponent :type "PrimitiveComponent Object Reference") (OtherActor :type "Actor Object Reference") (OtherComp :type "PrimitiveComponent Object Reference") (OtherBodyIndex :type Integer) (bFromSweep :type Boolean) (SweepResult :type "HitResult Structure (by ref)"))
  ;[0.05127 0.05127 0.05127] Takedown Radius
  (bind _asbp_third_person_character (cast `/Game/ThirdPerson/Blueprints/BP_ThirdPersonCharacter` OtherActor))
  (set `self.AI BP` _asbp_third_person_character)
  (`SceneComponent.SetVisibility` (`self.Takedown Widget`) true false))

(event `self.Takedown Widget.OnComponentEndOverlap`
  (params (OverlappedComponent :type "PrimitiveComponent Object Reference") (OtherActor :type "Actor Object Reference") (OtherComp :type "PrimitiveComponent Object Reference") (OtherBodyIndex :type Integer))
  ;[0.05127 0.05127 0.05127] Takedown Radius
  (cast `/Game/ThirdPerson/Blueprints/BP_ThirdPersonCharacter` OtherActor)
  (`SceneComponent.SetVisibility` (`self.Takedown Widget`) false false))

(event `self.ReceiveAnyDamage`
  (params (Damage :type "Float (single-precision)") (DamageType :type "DamageType Object Reference") (InstigatedBy :type "Controller Object Reference") (DamageCauser :type "Actor Object Reference"))
  (bind _hitanims (`self.HitAnims`))
  ;[0.05127 0.05127 0.05127] Recieve Damage
  (`self.Stop Combo`)
  (`self.PlayAnimMontage` (`|GetArrayItem` _hitanims (`KismetMathLibrary.RandomIntegerInRange` 0 (- (`KismetArrayLibrary.Array_Length` _hitanims) 1))))
  (bind _asbp_third_person_character (cast `/Game/ThirdPerson/Blueprints/BP_ThirdPersonCharacter` (`GameplayStatics.GetPlayerCharacter` 0)))
  (`self.LaunchCharacter` (* (`KismetMathLibrary.GetForwardVector` (`self.K2_GetActorRotation` _asbp_third_person_character)) 500.0))
  (`GameplayStatics.PlaySoundAtLocation` "/Game/Audio/Grunts-Hits/GetHitSFX.GetHitSFX" (`self.K2_GetActorLocation`) (struct) 1.0 (`KismetMathLibrary.RandomFloatInRange` -1.5 0.5) 0.0 "/Game/Audio/SA_Character.SA_Character" null null null)
  (bind _isplayerdead_ (`/Game/ThirdPerson/Blueprints/BPC_PlayerStats.Decrease Health` (`self.BPC_PlayerStats`) Damage))
  (if _isplayerdead_
    (`PrimitiveComponent.SetCollisionObjectType` (`self.Mesh`) "ECC_PhysicsBody")
    (`PrimitiveComponent.SetSimulatePhysics` (`self.Mesh`) true)
    (`GameplayStatics.PlaySoundAtLocation` "/Game/Audio/Grunts-Hits/MS_Death.MS_Death" (`self.K2_GetActorLocation`) (struct) 1.0 1.0 0.0 null null null null)
    (`SceneComponent.SetVisibility` (`self.Health Bar Widget`) false false)
    (`ActorComponent.K2_DestroyComponent` (`self.CapsuleComponent`))
    (`ActorComponent.K2_DestroyComponent` (`self.Assassination Radius`))))

(event `Melee Ataack Combo Call From BT`
  ;[0.05127 0.05127 0.05127] Combo System
  ;;[0.05127 0.05127 0.05127] Attack Click
  (if (`self.can Attack?`)
    (`self.MeleeAttack`)))

(event `Attack 1`
  ;[0.05127 0.05127 0.05127] Combo System
  ;;[0.05127 0.05127 0.05127] Attack 1
  (`/Engine/EditorBlueprintResources/StandardMacros.DoOnce` false :!label _label
    (:`Completed`
      (`KismetSystemLibrary.Delay` 0.1)
      (`|PlayMontage` (`self.Mesh`) "/Game/Characters/PlayerCharacter/Animations/Attacks/Punching_UE_Montage.Punching_UE_Montage"
        (:`then`
          (set `self.Attack Index` 1)
          (goto _label :!via `Reset`))))))

(event `MeleeAttack`
  ;[0.05127 0.05127 0.05127] Combo System
  ;;[0.05127 0.05127 0.05127] Melee Attack
  (if (`self.Is Attacking`)
    (set `self.saveAttack?` true)
    (else
      (set `self.Is Attacking` true)
      (switch `int` (`self.Attack Index`) :!label _label_2
        (:`0`
          (`self.Attack 1`))
        (:`1`
          (`self.Attack 2`))
        (:`2`
          (`self.Attack 3`))))))

(event `Attack 2`
  ;[0.05127 0.05127 0.05127] Combo System
  ;;[0.05127 0.05127 0.05127] Attack 2
  (`/Engine/EditorBlueprintResources/StandardMacros.DoOnce` false :!label _label_3
    (:`Completed`
      (`KismetSystemLibrary.Delay` 0.1)
      (`|PlayMontage` (`self.Mesh`) "/Game/Characters/PlayerCharacter/Animations/Attacks/LeftHook_UE_Montage.LeftHook_UE_Montage"
        (:`then`
          (set `self.Attack Index` 2)
          (goto _label_3 :!via `Reset`))))))

(event `Melee Attack Combo`
  ;[0.05127 0.05127 0.05127] Combo System
  ;;[0.05127 0.05127 0.05127] Combo Continue
  (if (`self.saveAttack?`)
    (set `self.saveAttack?` false)
    (goto _label_2)
    (else
      (`self.Stop Combo`))))

(event `Attack 3`
  ;[0.05127 0.05127 0.05127] Combo System
  ;;[0.05127 0.05127 0.05127] Attack 3
  (`/Engine/EditorBlueprintResources/StandardMacros.DoOnce` false :!label _label_4
    (:`Completed`
      (`KismetSystemLibrary.Delay` 0.1)
      (`|PlayMontage` (`self.Mesh`) "/Game/Characters/PlayerCharacter/Animations/Attacks/RightHook_UE_Montage.RightHook_UE_Montage"
        (:`then`
          (set `self.Attack Index` 3)
          (goto _label_4 :!via `Reset`))))))

(event `Stop Combo`
  ;[0.05127 0.05127 0.05127] Combo System
  ;;[0.05127 0.05127 0.05127] Stop Combo/Attack
  (set `self.Is Attacking` false)
  (set `self.Attack Index` 0))

(event `Attack 4`
  ;[0.05127 0.05127 0.05127] Combo System
  ;;[0.05127 0.05127 0.05127] Attack 4 (Not using atm)
  (`/Engine/EditorBlueprintResources/StandardMacros.DoOnce` false
    (:`Completed`
      (`KismetSystemLibrary.Delay` 0.1)
      (`|PlayMontage` (`self.Mesh`) "/Game/Characters/PlayerCharacter/Animations/Attacks/Kick_Montage.Kick_Montage"
        (:`then`
          (set `self.Attack Index` 4))))))

(event `Start Melee Trace`
  (bind _returnvalue (`KismetSystemLibrary.K2_SetTimerDelegate` (delegate `Melee Trace Loop`) 0.1 true))
  (set `self.MeleeTraceLoop` _returnvalue))

(event `Melee Trace Loop`
  (bind _returnvalue (`SceneComponent.GetSocketLocation` (`Character.Mesh` (`self.AI BP`)) "foot_r"))
  (bind _returnvalue_2 (`SceneComponent.GetSocketLocation` (`Character.Mesh` (`self.AI BP`)) "hand_r"))
  (bind _returnvalue_3 (`SceneComponent.GetSocketLocation` (`Character.Mesh` (`self.AI BP`)) "hand_l"))
  (`|ExecutionSequence`
    (:`then_0`
      ;[0.05127 0.05127 0.05127] Right Hand Tracking
      (bind (_outhit _returnvalue_4) (`KismetSystemLibrary.SphereTraceSingle` :`Start` _returnvalue_2 :`End` _returnvalue_2 :`Radius` 12.0 :`TraceChannel` "TraceTypeQuery1" :`DrawDebugType` "ForDuration"))
      (if _returnvalue_4
        (bind (_bblockinghit _binitialoverlap _time _distance _location _impactpoint _normal _impactnormal _physmat _hitactor) (`GameplayStatics.BreakHitResult` _outhit))
        (if (`self.ActorHasTag` _hitactor "Damageable")
          (`/Engine/EditorBlueprintResources/StandardMacros.DoOnce` false :!label _label_5
            (:`Completed`
              (`GameplayStatics.ApplyDamage` _hitactor 10.0)
              (`self.Play Melee Hit Sounds`)
              (`GameplayStatics.SpawnEmitterAtLocation` "/Game/VFX/Particles/Blood/P_Blood_Splat_Cone.P_Blood_Splat_Cone" _location (`KismetMathLibrary.MakeRotFromXY` _normal _normal) (0.4 0.4 0.4) true "AutoRelease")
              (`KismetSystemLibrary.Delay` 0.5)
              (goto _label_5 :!via `Reset`))))))
    (:`then_1`
      ;[0.05127 0.05127 0.05127] Left Hand Tracking
      (bind (_outhit_2 _returnvalue_5) (`KismetSystemLibrary.SphereTraceSingle` :`Start` _returnvalue_3 :`End` _returnvalue_3 :`Radius` 12.0 :`TraceChannel` "TraceTypeQuery1" :`DrawDebugType` "ForDuration"))
      (if _returnvalue_5
        (bind (_bblockinghit_2 _binitialoverlap_2 _time_2 _distance_2 _location_2 _impactpoint_2 _normal_2 _impactnormal_2 _physmat_2 _hitactor_2) (`GameplayStatics.BreakHitResult` _outhit_2))
        (if (`self.ActorHasTag` _hitactor_2 "Damageable")
          (`/Engine/EditorBlueprintResources/StandardMacros.DoOnce` false :!label _label_6
            (:`Completed`
              (`GameplayStatics.ApplyDamage` _hitactor_2 10.0)
              (`self.Play Melee Hit Sounds`)
              (`GameplayStatics.SpawnEmitterAtLocation` "/Game/VFX/Particles/Blood/P_Blood_Splat_Cone.P_Blood_Splat_Cone" _location_2 (`KismetMathLibrary.MakeRotFromXY` _normal_2 _normal_2) (0.4 0.4 0.4) true "AutoRelease")
              (`KismetSystemLibrary.Delay` 0.5)
              (goto _label_6 :!via `Reset`))))))
    (:`then_2`
      ;[0.05127 0.05127 0.05127] Right Foot Tracking
      (bind (_outhit_3 _returnvalue_6) (`KismetSystemLibrary.SphereTraceSingle` :`Start` _returnvalue :`End` _returnvalue :`Radius` 12.0 :`TraceChannel` "TraceTypeQuery1" :`DrawDebugType` "ForDuration"))
      (if _returnvalue_6
        (bind (_bblockinghit_3 _binitialoverlap_3 _time_3 _distance_3 _location_3 _impactpoint_3 _normal_3 _impactnormal_3 _physmat_3 _hitactor_3) (`GameplayStatics.BreakHitResult` _outhit_3))
        (if (`self.ActorHasTag` _hitactor_3 "Damageable")
          (`/Engine/EditorBlueprintResources/StandardMacros.DoOnce` false :!label _label_7
            (:`Completed`
              (`GameplayStatics.ApplyDamage` _hitactor_3 10.0)
              (`self.Play Melee Hit Sounds`)
              (`GameplayStatics.SpawnEmitterAtLocation` "/Game/VFX/Particles/Blood/P_Blood_Splat_Cone.P_Blood_Splat_Cone" _location_3 (`KismetMathLibrary.MakeRotFromXY` _normal_3 _normal_3) (0.4 0.4 0.4) true "AutoRelease")
              (`KismetSystemLibrary.Delay` 0.5)
              (goto _label_7 :!via `Reset`))))))))

(event `Stop Melee Trace`
  (`KismetSystemLibrary.K2_ClearAndInvalidateTimerHandle` (`self.MeleeTraceLoop`)))

(event `Play Melee Hit Sounds`
  ;[0.05127 0.05127 0.05127] Play Melee Hit Sounds
  (`GameplayStatics.PlaySoundAtLocation` "/Game/Audio/MeleeHits/MS_Hit.MS_Hit" (`self.K2_GetActorLocation` (`self.GetOwner`)) (struct) 1.0 1.0 0.0 "/Game/Audio/SA_Character.SA_Character" null null null))

(event `Investigate Icon`
  (bind _investigate_widget (`self.Investigate Widget`))
  (`/Engine/EditorBlueprintResources/StandardMacros.FlipFlop`
    (:`A`
      (`SceneComponent.SetVisibility` _investigate_widget true false))
    (:`B`
      (`SceneComponent.SetVisibility` _investigate_widget false false))))

(fn `Attack`
  (returns (AnimationDuration :type "Float (double-precision)"))
  (`self.Melee Ataack Combo Call From BT`)
  (return 0.4))

(fn `Stealth Back Assassin`
  (returns (`REF Location` :type "Vector Structure") (`Assassin Rotation` :type "Rotator Structure"))
  (bind (_returnvalue_x _returnvalue_y _returnvalue_z) (`KismetMathLibrary.BreakVector` (`SceneComponent.K2_GetComponentLocation` (`self.Assassin REF`))))
  (`self.PlayAnimMontage` "/Game/Characters/PlayerCharacter/Animations/Assassinations/Paired_SneakNeckBreak_Vic_Montage.Paired_SneakNeckBreak_Vic_Montage")
  (`self.Ragdoll`)
  (`SceneComponent.SetVisibility` (`self.Takedown Widget`) false false)
  (return (`KismetMathLibrary.MakeVector` _returnvalue_x _returnvalue_y _returnvalue_z) (`self.K2_GetActorRotation`)))

(fn `UserConstructionScript`)